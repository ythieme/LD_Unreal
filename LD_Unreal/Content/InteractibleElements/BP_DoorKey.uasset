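; BP_DoorKey is an interactable locked door that carries its own key pickup in the same actor.
; Overlapping the key or door trigger toggles prompts and Interact input; the key also gets a custom-depth highlight.
; A single Interact event picks up the key, unlocks the door, or opens and closes it through rotation timelines, based on state booleans.
; The player's local-space side sets the swing direction and prompt placement.
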(event OnComponentBeginOverlap(Trigger)
  (params (OverlappedComponent :type Primitive%20Component%20Object%20Reference) (OtherActor :type Actor%20Object%20Reference) (OtherComp :type Primitive%20Component%20Object%20Reference) (OtherBodyIndex :type Integer) (bFromSweep :type Boolean) (SweepResult :type Hit%20Result%20Structure%20%28by%20ref%29))
  (bind _input (Variables|Default|GetInput))
  (bind _input_2 (Variables|Default|GetInput))
  (bind _input_3 (Variables|Default|GetInput))
  (bind _input_4 (Variables|Default|GetInput))
  ;[1 1 1] Activation des Inputs et Apparition du texte quand le Player est dans le Trigger de la Porte. Si la porte est "Lock", alors la porte ne peut pas s'ouvrir (input désactivé)
  (Variables|Default|SetDirection (> (.X (Math|Vector|BreakVector (Math|Vector|UnrotateVector (- (Transformation|GetActorLocation) (Transformation|GetActorLocation (Game|GetPlayerCharacter 0))) (Transformation|GetActorRotation)))) 0.0))
  (Audio|Components|Audio|Stop (Variables|Default|GetClose))
  (if (Variables|Default|GetisUnlock)
    (if (Variables|Default|GetisOpen)
      (Rendering|Components|TextRender|SetText _input (Variables|Default|GetTextClose))
      (else
        (Rendering|Components|TextRender|SetText _input (Variables|Default|GetTextOpen))))
    (if (Variables|Default|GetDirection) :!label _label
      (Transformation|SetRelativeLocationAndRotation _input_3 "-30.000000,30.000000,90.000000" "0.000000,180.000000,0.000000" false false)
      (else
        (Transformation|SetRelativeLocationAndRotation _input_3 "30.000000,30.000000,90.000000" "0, 0, 0" false false)))
    (Rendering|SetVisibility (Variables|Default|GetInput) true false)
    (Input|EnableInput (Game|GetPlayerController 0))
    (elif (Variables|Default|GethasKey)
      (Rendering|Components|TextRender|SetText _input_4 (Variables|Default|GetTextUseKey))
      (Rendering|SetVisibility _input_4 true false)
      (goto _label)
      (else
        (Rendering|Components|TextRender|SetText (Variables|Default|GetInput) (Variables|Default|GetTextLock))
        (if (Variables|Default|GetDirection)
          (Transformation|SetRelativeLocationAndRotation _input_2 "-30.000000,30.000000,90.000000" "0.000000,180.000000,0.000000" false false)
          (else
            (Transformation|SetRelativeLocationAndRotation _input_2 "30.000000,30.000000,90.000000" "0, 0, 0" false false)))
        (Rendering|SetVisibility _input_2 true false)))))

(event OnComponentEndOverlap(Trigger)
  (params (OverlappedComponent :type Primitive%20Component%20Object%20Reference) (OtherActor :type Actor%20Object%20Reference) (OtherComp :type Primitive%20Component%20Object%20Reference) (OtherBodyIndex :type Integer))
  ;[1 1 1] Activation des Inputs et Apparition du texte quand le Player est dans le Trigger de la Porte. Si la porte est "Lock", alors la porte ne peut pas s'ouvrir (input désactivé)
  (Audio|Components|Audio|Stop (Variables|Default|GetOpen))
  (Rendering|SetVisibility (Variables|Default|GetInput) false false)
  (Input|DisableInput (Game|GetPlayerController 0)))

(event OnComponentBeginOverlap(KeyTrigger)
  (params (OverlappedComponent :type Primitive%20Component%20Object%20Reference) (OtherActor :type Actor%20Object%20Reference) (OtherComp :type Primitive%20Component%20Object%20Reference) (OtherBodyIndex :type Integer) (bFromSweep :type Boolean) (SweepResult :type Hit%20Result%20Structure%20%28by%20ref%29))
  ;[1 1 1] Key
  (Rendering|SetVisibility (Variables|Default|GetKeyInput) true false)
  (Input|EnableInput (Game|GetPlayerController 0))
  (Rendering|SetRenderCustomDepth (Variables|Default|GetKey) true))

(event OnComponentEndOverlap(KeyTrigger)
  (params (OverlappedComponent :type Primitive%20Component%20Object%20Reference) (OtherActor :type Actor%20Object%20Reference) (OtherComp :type Primitive%20Component%20Object%20Reference) (OtherBodyIndex :type Integer))
  ;[1 1 1] Key
  (Rendering|SetVisibility (Variables|Default|GetKeyInput) false false)
  (Input|DisableInput (Game|GetPlayerController 0))
  (Rendering|SetRenderCustomDepth (Variables|Default|GetKey) false))

(event Input|ActionEvents|InputActionInteract
  (params (Key :type Key%20Structure :default "None"))
  (bind _sm_door (Variables|Default|GetSM_Door))
  (bind _input (Variables|Default|GetInput))
  (bind _sm_door_2 (Variables|Default|GetSM_Door))
  ;[1 1 1] Quand Input "Interact" est appuyé : Ouvre la Porte quand elle est fermée, Ferme la porte quand elle est ouverte. Le texte change en fonction de l'interaction possible
  (:Pressed
    (if (Variables|Default|GetisUnlock)
      (if (Variables|Default|GetisOpen)
        (bind _rotation (Timeline|Close PlayFromStart)
          (:Update
            (Variables|Default|SetisOpen false)
            (Transformation|SetRelativeRotation _sm_door_2 (Math|Rotator|Lerp(Rotator) (Variables|/Script/Engine.SceneComponent|GetRelativeRotation _sm_door_2) "0, 0, 0" _rotation true) false false)
            (Rendering|Components|TextRender|SetText _input (Variables|Default|GetTextOpen))))
        (else
          (bind _rotation_2 (Timeline|Open PlayFromStart)
            (:Update
              (Variables|Default|SetisOpen true)
              (Transformation|SetRelativeRotation _sm_door (Math|Rotator|Lerp(Rotator) (Variables|/Script/Engine.SceneComponent|GetRelativeRotation _sm_door) (Math|Rotator|MakeRotator 0.0 0.0 (Math|Float|SelectFloat -9e+01 9e+01 (Variables|Default|GetDirection))) _rotation_2 true) false false)
              (Rendering|Components|TextRender|SetText _input (Variables|Default|GetTextClose))))))
      (elif (Variables|Default|GethasKey)
        (Variables|Default|SetisUnlock true)
        (else
          ;[1 1 1] C'est ultra moche, mais si la porte n'est pas débloquée "unblock", alors l'input E ramasse la clé donc passe le booléen "hasKey" a true, et fait disparaitre la clé
          (Variables|Default|SethasKey true)
          (Components|DestroyComponent (Variables|Default|GetKeyTrigger))
          (Components|DestroyComponent (Variables|Default|GetKeyInput))
          (Components|DestroyComponent (Variables|Default|GetKey)))))))

(fn ConstructionScript)