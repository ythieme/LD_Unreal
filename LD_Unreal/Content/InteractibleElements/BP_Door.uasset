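; BP_Door is an interactive door that the player opens and closes with the Interact input, starting in the state set by IsOpen.
; A trigger toggles input and an open/close text prompt, and picks the prompt's side and swing direction from the player's position so the door opens away from them.
; Open and Close timelines lerp the door mesh yaw and update state and text, with a sound spawned on each interaction.
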(event OnComponentBeginOverlap(Trigger)
  (params (OverlappedComponent :type Primitive%20Component%20Object%20Reference) (OtherActor :type Actor%20Object%20Reference) (OtherComp :type Primitive%20Component%20Object%20Reference) (OtherBodyIndex :type Integer) (bFromSweep :type Boolean) (SweepResult :type Hit%20Result%20Structure%20%28by%20ref%29))
  (bind _input (Variables|Default|GetInput))
  (bind _input_2 (Variables|Default|GetInput))
  ;[1 1 1] Activation des Inputs et Apparition du texte quand le Player est dans le Trigger de la Porte.
  (Variables|Default|SetDirection (> (.X (Math|Vector|BreakVector (Math|Vector|UnrotateVector (- (Transformation|GetActorLocation) (Transformation|GetActorLocation (Game|GetPlayerCharacter 0))) (Transformation|GetActorRotation)))) 0.0))
  (Audio|Components|Audio|Stop (Variables|Default|GetClose))
  (if (Variables|Default|GetisOpen)
    (Rendering|Components|TextRender|SetText _input (Variables|Default|GetTextClose))
    (else
      (Rendering|Components|TextRender|SetText _input (Variables|Default|GetTextOpen))))
  (if (Variables|Default|GetDirection)
    (Transformation|SetRelativeLocationAndRotation _input_2 "-30.000000,30.000000,90.000000" "0.000000,180.000000,0.000000" false false)
    (else
      (Transformation|SetRelativeLocationAndRotation _input_2 "30.000000,30.000000,90.000000" "0, 0, 0" false false)))
  (Rendering|SetVisibility (Variables|Default|GetInput) true false)
  (Input|EnableInput (Game|GetPlayerController 0)))

(event OnComponentEndOverlap(Trigger)
  (params (OverlappedComponent :type Primitive%20Component%20Object%20Reference) (OtherActor :type Actor%20Object%20Reference) (OtherComp :type Primitive%20Component%20Object%20Reference) (OtherBodyIndex :type Integer))
  ;[1 1 1] Activation des Inputs et Apparition du texte quand le Player est dans le Trigger de la Porte.
  (Audio|Components|Audio|Stop (Variables|Default|GetOpen))
  (Rendering|SetVisibility (Variables|Default|GetInput) false false)
  (Input|DisableInput (Game|GetPlayerController 0)))

(event EventBeginPlay
  ;[1 1 1] Dès le début, selon isOpen True ou False, la porte est ouverte ou non
  (if (Variables|Default|GetisOpen)
    (Components|Timeline|PlayfromStart (Variables|Default|GetOpen))
    (else
      (Components|Timeline|PlayfromStart (Variables|Default|GetClose)))))

(event Input|ActionEvents|InputActionInteract
  (params (Key :type Key%20Structure :default "None"))
  (bind _sm_door (Variables|Default|GetSM_Door))
  (bind _input (Variables|Default|GetInput))
  (bind _sm_door_2 (Variables|Default|GetSM_Door))
  ;[1 1 1] Quand Input "Interact" est appuyé : Ouvre la Porte quand elle est fermée, Ferme la porte quand elle est ouverte. Le texte change en fonction de l'interaction possible
  (:Pressed
    (if (Variables|Default|GetisOpen)
      (Audio|SpawnSoundatLocation "/Game/Draft/Sound/CloseDoor_Cue.CloseDoor_Cue" (Transformation|GetWorldLocation (Variables|Default|GetSM_DoorFrame)) "0, 0, 0" 1.0 1.0 0.0 0 0)
      (bind _rotation (Timeline|Close PlayFromStart)
        (:Update
          (Variables|Default|SetisOpen false)
          (Transformation|SetRelativeRotation _sm_door_2 (Math|Rotator|Lerp(Rotator) (Variables|/Script/Engine.SceneComponent|GetRelativeRotation _sm_door_2) "0, 0, 0" _rotation true) false false)
          (Rendering|Components|TextRender|SetText _input (Variables|Default|GetTextOpen))))
      (else
        (Audio|SpawnSoundatLocation "/Game/Draft/Sound/OpenDoor_Cue.OpenDoor_Cue" (Transformation|GetWorldLocation (Variables|Default|GetSM_DoorFrame)) "0, 0, 0" 1.0 1.0 0.0 0 0)
        (bind _rotation_2 (Timeline|Open PlayFromStart)
          (:Update
            (Variables|Default|SetisOpen true)
            (Transformation|SetRelativeRotation _sm_door (Math|Rotator|Lerp(Rotator) (Variables|/Script/Engine.SceneComponent|GetRelativeRotation _sm_door) (Math|Rotator|MakeRotator 0.0 0.0 (Math|Float|SelectFloat -9e+01 9e+01 (Variables|Default|GetDirection))) _rotation_2 true) false false)
            (Rendering|Components|TextRender|SetText _input (Variables|Default|GetTextClose))))))))

(fn ConstructionScript)