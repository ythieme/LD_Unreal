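; BP_KeypadDoor is a door that stays locked until the correct code is entered on its keypad widget.
; It binds to the widget's CodeEntered event, and CheckCode unlocks the door on a match, turning light and lock color green, or resets the entry.
; Overlapping the trigger plays a timeline that swings the unlocked door open, and leaving plays one that closes it.
; The keypad trigger's overlap events are empty.
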(event OnComponentBeginOverlap(KeypadTrigger)
  (params (OverlappedComponent :type Primitive%20Component%20Object%20Reference) (OtherActor :type Actor%20Object%20Reference) (OtherComp :type Primitive%20Component%20Object%20Reference) (OtherBodyIndex :type Integer) (bFromSweep :type Boolean) (SweepResult :type Hit%20Result%20Structure%20%28by%20ref%29))
  ;[1 1 1] Quand on entre dans le trigger du Keypad, on peut cliquer
)

(event OnComponentEndOverlap(Trigger)
  (params (OverlappedComponent :type Primitive%20Component%20Object%20Reference) (OtherActor :type Actor%20Object%20Reference) (OtherComp :type Primitive%20Component%20Object%20Reference) (OtherBodyIndex :type Integer))
  (bind _sm_door (Variables|Default|GetSM_Door))
  ;[1 1 1] Quand Input "Interact" est appuyé : Ouvre la Porte quand elle est fermée, Ferme la porte quand elle est ouverte. Le texte change en fonction de l'interaction possible
  (bind _rotation (Timeline|Close PlayFromStart)
    (:Update
      (Transformation|SetRelativeRotation _sm_door (Math|Rotator|Lerp(Rotator) (Variables|/Script/Engine.SceneComponent|GetRelativeRotation _sm_door) "0, 0, 0" _rotation true) false false))))

(event OnComponentBeginOverlap(Trigger)
  (params (OverlappedComponent :type Primitive%20Component%20Object%20Reference) (OtherActor :type Actor%20Object%20Reference) (OtherComp :type Primitive%20Component%20Object%20Reference) (OtherBodyIndex :type Integer) (bFromSweep :type Boolean) (SweepResult :type Hit%20Result%20Structure%20%28by%20ref%29))
  (bind _sm_door (Variables|Default|GetSM_Door))
  ;[1 1 1] Quand Input "Interact" est appuyé : Ouvre la Porte quand elle est fermée, Ferme la porte quand elle est ouverte. Le texte change en fonction de l'interaction possible
  (if (not (Variables|Default|GetisLocked))
    (bind _rotation (Timeline|Open PlayFromStart)
      (:Update
        (Transformation|SetRelativeRotation _sm_door (Math|Rotator|Lerp(Rotator) (Variables|/Script/Engine.SceneComponent|GetRelativeRotation _sm_door) "0.000000,90.000000,0.000000" _rotation true) false false)))))

(event OnComponentEndOverlap(KeypadTrigger)
  (params (OverlappedComponent :type Primitive%20Component%20Object%20Reference) (OtherActor :type Actor%20Object%20Reference) (OtherComp :type Primitive%20Component%20Object%20Reference) (OtherBodyIndex :type Integer))
  ;[1 1 1] Quand on entre dans le trigger du Keypad, on peut cliquer
)

(event EventBeginPlay
  (bind _aswbp_keypad_ui (Utilities|Casting|CastToWBP_KeypadUI (UserInterface|GetUserWidgetObject (Variables|Default|GetKeypadWidget))))
  (bind _output_get (Variables|Default|SetKeypad_UI _aswbp_keypad_ui))
  (EventDispatchers|BindEventtoCodeEntered _output_get (EventDispatchers|CreateEvent :!event CheckCode))
  (Rendering|Material|SetMaterial (Variables|Default|GetLight) 0 "/Game/Materials/MI_DoorLightRd.MI_DoorLightRd"))

(fn ConstructionScript)

(fn CheckCode
  (params (Codeentered :type String) (KeypadUI :type WBP%20Keypad%20UI%20Object%20Reference))
  (if (Utilities|Enum|Equal(Enum) Codeentered (Variables|Default|GetCorrectCode))
    (Variables|Default|SetisLocked false)
    (Variables|/Game/InteractibleElements/WBP_KeypadUI.WBP_KeypadUI_C|SetCurrentCode (Variables|Default|GetKeypad_UI) "")
    (Rendering|Material|SetMaterial (Variables|Default|GetLight) 0 "/Game/Materials/MI_DoorLightGr.MI_DoorLightGr")
    (Class|Border|SetBrushColor (Variables|/Game/InteractibleElements/WBP_KeypadUI.WBP_KeypadUI_C|GetLockColor (Variables|Default|GetKeypad_UI)) "(R=0.182582,G=0.710069,B=0.060405,A=1.000000)")
    (else
      (Variables|/Game/InteractibleElements/WBP_KeypadUI.WBP_KeypadUI_C|SetCurrentCode (Variables|Default|GetKeypad_UI) "")
      (Rendering|Components|TextRender|SetText (Variables|/Game/InteractibleElements/WBP_KeypadUI.WBP_KeypadUI_C|GetCodeText (Variables|Default|GetKeypad_UI)) "----"))))