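; BP_MonsterInVent is a one-shot scare actor that fakes a monster moving through a vent with footstep sounds.
; Overlapping its trigger destroys the trigger after a short delay and plays a timeline that lerps a static mesh from its start position by a Distance offset.
; The first timeline update starts a looping timer spawning footstep sounds attached to that mesh, then destroys the actor after a set time.
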(event OnComponentBeginOverlap(Trigger)
  (params (OverlappedComponent :type Primitive%20Component%20Object%20Reference) (OtherActor :type Actor%20Object%20Reference) (OtherComp :type Primitive%20Component%20Object%20Reference) (OtherBodyIndex :type Integer) (bFromSweep :type Boolean) (SweepResult :type Hit%20Result%20Structure%20%28by%20ref%29))
  ;[1 1 1] Le "monstre" se déplace du StartPos au EndPos et tant qu'il se déplace, il joue le son de marche
  (Utilities|FlowControl|Delay 0.2)
  (Components|DestroyComponent (Variables|Default|GetTrigger))
  (bind _monstermovement (Timeline|MonsterPosition PlayFromStart)
    (:Update
      (Transformation|SetWorldLocation (Variables|Default|GetStaticMesh) (Math|Vector|Lerp(Vector) (Variables|Default|GetStartPos) (Variables|Default|GetEndPos) _monstermovement) false false)
      (Utilities|FlowControl|DoOnce false
        (:Completed
          (Utilities|Time|SetTimerbyEvent (delegate Custom|MonsterFootSteps) (Variables|Default|GetFootStepInterval) true)
          (Utilities|FlowControl|Delay (Variables|Default|GetTime))
          (Actor|DestroyActor))))))

(event Custom|MonsterFootSteps
  ;[1 1 1] Joue le son des pas du monstre
  (Audio|SpawnSoundAttached "/Game/Draft/Sound/FootstepsMonster/SC_FootStepsMonster.SC_FootStepsMonster" (Variables|Default|GetStaticMesh) "None" "0, 0, 0" "0, 0, 0" "KeepRelativeOffset" false 1.0 1.0 0.0 0 0))

(event EventBeginPlay
  ;[1 1 1] Au début du niveau, on détermine le point de départ et le point d'arrivée du point que le son suivra. La distance à parcourir est à déterminer
  (bind _output_get (Variables|Default|SetStartPos (Transformation|GetWorldLocation (Variables|Default|GetStaticMesh))))
  (Variables|Default|SetEndPos (+ _output_get (Variables|Default|GetDistance))))

(fn ConstructionScript)