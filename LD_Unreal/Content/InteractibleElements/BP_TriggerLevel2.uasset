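; Level-transition trigger that swaps tagged sets of actors when its Trigger component is overlapped.
; BeginPlay hides and disables collision on NewTag actors and gathers OldTag actors.
; Overlap, with no check on the overlapping actor, reveals the new and destroys the old, then removes the trigger.
; The overlap reads the BeginPlay loops' element outputs without looping again, so it does not iterate over either set.
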(event OnComponentBeginOverlap(Trigger)
  (params (OverlappedComponent :type Primitive%20Component%20Object%20Reference) (OtherActor :type Actor%20Object%20Reference) (OtherComp :type Primitive%20Component%20Object%20Reference) (OtherBodyIndex :type Integer) (bFromSweep :type Boolean) (SweepResult :type Hit%20Result%20Structure%20%28by%20ref%29))
  ;[1 1 1] Quand le joueur passe dans le trigger, ça fait disparaître tous les anciens actors
  (Rendering|SetActorHiddenInGame (stale EventBeginPlay _array_element) false)
  (Collision|SetActorEnableCollision (stale EventBeginPlay _array_element) true)
  (Actor|DestroyActor (stale EventBeginPlay _array_element_2))
  (Components|DestroyComponent (Variables|Default|GetTrigger)))

(event EventBeginPlay
  ;[1 1 1] Au lancement de l'objet, il récupère tous les actors avec les tags indiqués : le tag pour les actors qui vont disparaître et le tag de ceux qui vont apparaître (les cache et désactive en même temps)
  (bind _outactors (Actor|GetAllActorswithTag (Variables|Default|GetNewTag)))
  (for _array_element _outactors
    (Collision|SetActorEnableCollision _array_element false)
    (Rendering|SetActorHiddenInGame _array_element true))
  (bind _outactors_2 (Actor|GetAllActorswithTag (Variables|Default|GetOldTag)))
  (for _array_element_2 _outactors_2
    _))

(fn ConstructionScript)