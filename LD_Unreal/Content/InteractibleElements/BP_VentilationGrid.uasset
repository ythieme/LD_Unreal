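; BP_VentilationGrid is an interactible ventilation grid that the player can open and remove.
; Its trigger overlap toggles the Input prompt and enables or disables player 0's input on the actor.
; Pressing Interact plays the OpenGrid timeline, which incrementally offsets the frame mesh along local Y.
; A delay started from the timeline's update stops it after OpenDuration and destroys the mesh component.
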(event OnComponentBeginOverlap(Trigger)
  (params (OverlappedComponent :type Primitive%20Component%20Object%20Reference) (OtherActor :type Actor%20Object%20Reference) (OtherComp :type Primitive%20Component%20Object%20Reference) (OtherBodyIndex :type Integer) (bFromSweep :type Boolean) (SweepResult :type Hit%20Result%20Structure%20%28by%20ref%29))
  ;[1 1 1] Si le Player est dans le Trigger, il peut appuyer sur l'input pour ouvrir la grille. Le texte s'affiche
  (Rendering|SetVisibility (Variables|Default|GetInput) true false)
  (Input|EnableInput (Game|GetPlayerController 0)))

(event OnComponentEndOverlap(Trigger)
  (params (OverlappedComponent :type Primitive%20Component%20Object%20Reference) (OtherActor :type Actor%20Object%20Reference) (OtherComp :type Primitive%20Component%20Object%20Reference) (OtherBodyIndex :type Integer))
  ;[1 1 1] Si le Player est dans le Trigger, il peut appuyer sur l'input pour ouvrir la grille. Le texte s'affiche
  (Rendering|SetVisibility (Variables|Default|GetInput) false false)
  (Input|DisableInput (Game|GetPlayerController 0)))

(event Input|ActionEvents|InputActionInteract
  (params (Key :type Key%20Structure :default "None"))
  (bind _sm_windowframe1 (Variables|Default|GetSM_WindowFrame1))
  (bind _relativelocation (Variables|/Script/Engine.SceneComponent|GetRelativeLocation _sm_windowframe1))
  ;[1 1 1] Quand le joueur appuie sur input "Interact", la grille vacille pendant quelques secondes puis disparait elle disparait
  (:Pressed
    (bind _move (Timeline|OpenGrid PlayFromStart)
      (:Update
        (Transformation|SetRelativeLocation _sm_windowframe1 (Math|Vector|Lerp(Vector) _relativelocation (+ _relativelocation "0.000000,0.100000,0.000000") _move) false false)
        (Utilities|FlowControl|Delay (Variables|Default|GetOpenDuration))
        (Audio|Components|Audio|Stop (Variables|Default|GetOpenGrid))
        (Components|DestroyComponent (Variables|Default|GetSM_WindowFrame1))))))

(fn ConstructionScript)