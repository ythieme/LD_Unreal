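; BP_MonsterShadow is a one-shot scare that places a monster mesh at the player, intended behind them so its shadow falls in front.
; Overlapping its trigger moves the mesh along the camera's forward vector by Distance, at world Z zero, matches the camera's yaw and shows it.
; Tick then hides the mesh once the camera turns over 90 degrees from that facing, destroying the actor shortly after.
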(event OnComponentBeginOverlap(TriggerActivate)
  (params (OverlappedComponent :type Primitive%20Component%20Object%20Reference) (OtherActor :type Actor%20Object%20Reference) (OtherComp :type Primitive%20Component%20Object%20Reference) (OtherBodyIndex :type Integer) (bFromSweep :type Boolean) (SweepResult :type Hit%20Result%20Structure%20%28by%20ref%29))
  (bind _returnvalue (Game|GetPlayerCameraManager 0))
  (bind _returnvalue_2 (Game|GetPlayerCharacter 0))
  (bind _distance (Variables|Default|GetDistance))
  (bind _returnvalue_3 (Transformation|GetActorForwardVector _returnvalue))
  (bind _returnvalue_4 (Transformation|GetActorLocation _returnvalue_2))
  (bind _returnvalue_5 (* _returnvalue_3 _distance))
  (bind _returnvalue_6 (+ _returnvalue_5 _returnvalue_4))
  (bind (_x _y) (Math|Vector|BreakVector _returnvalue_6))
  (Transformation|SetWorldLocationAndRotation (Variables|Default|GetSM_Monster) (Math|Vector|MakeVector _x _y 0.0) (Math|Rotator|MakeRotator 0.0 0.0 (.Yaw (Math|Rotator|BreakRotator (Math|Rotator|MakeRotationfromAxes (Transformation|GetActorForwardVector (Game|GetPlayerCameraManager 0)) "0, 0, 0" "0, 0, 0")))) false false)
  (Rendering|SetVisibility (Variables|Default|GetSM_Monster) true true)
  (Variables|Default|SetisVisible true))

(event EventTick
  (params (DeltaSeconds :type Float%20%28single-precision%29))
  (if (Variables|Default|GetisVisible)
    (if (< (Class|KismetMathLibrary|VectorCosineAngle2D (Math|Vector|GetForwardVector (Variables|Default|GetSM_Monster)) (Transformation|GetActorForwardVector (Game|GetPlayerCameraManager 0))) 0.0)
      (Rendering|SetVisibility (Variables|Default|GetSM_Monster) false false)
      (Utilities|FlowControl|Delay 0.2)
      (Actor|DestroyActor))))

(fn ConstructionScript)