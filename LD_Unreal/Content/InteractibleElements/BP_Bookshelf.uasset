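; BP_Bookshelf is an interactible bookshelf that slides to a new position when the player presses Interact nearby.
; Overlapping the Trigger shows the Input prompt, enables player input and highlights the Shelf through custom depth; leaving reverses all three.
; BeginPlay stores the actor location as start and adds the NewPos offset for the end.
; The MoveShelf timeline lerps the Shelf component between them, replaying from the start on every press.
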(event OnComponentBeginOverlap(Trigger)
  (params (OverlappedComponent :type Primitive%20Component%20Object%20Reference) (OtherActor :type Actor%20Object%20Reference) (OtherComp :type Primitive%20Component%20Object%20Reference) (OtherBodyIndex :type Integer) (bFromSweep :type Boolean) (SweepResult :type Hit%20Result%20Structure%20%28by%20ref%29))
  ;[1 1 1] Quand le joueur est proche de l'étagère, le texte s'affiche et il peut appuyer pour la déplacer
  (Rendering|SetVisibility (Variables|Default|GetInput) true false)
  (Input|EnableInput (Game|GetPlayerController 0))
  (Rendering|SetRenderCustomDepth (Variables|Default|GetShelf) true))

(event OnComponentEndOverlap(Trigger)
  (params (OverlappedComponent :type Primitive%20Component%20Object%20Reference) (OtherActor :type Actor%20Object%20Reference) (OtherComp :type Primitive%20Component%20Object%20Reference) (OtherBodyIndex :type Integer))
  ;[1 1 1] Quand le joueur est proche de l'étagère, le texte s'affiche et il peut appuyer pour la déplacer
  (Rendering|SetVisibility (Variables|Default|GetInput) false false)
  (Input|DisableInput (Game|GetPlayerController 0))
  (Rendering|SetRenderCustomDepth (Variables|Default|GetShelf) false))

(event EventBeginPlay
  ;[1 1 1] Au lancement de la Map, on défini la position de l'Actor et sa position d'arrivée
  (bind _output_get (Variables|Default|SetStartPos (Transformation|GetActorLocation)))
  (Variables|Default|SetEndPos (+ _output_get (Variables|Default|GetNewPos))))

(event Input|ActionEvents|InputActionInteract
  (params (Key :type Key%20Structure :default "None"))
  ;[1 1 1] Quand le Player appuie sur l'input "Interact", l'étagère se déplace
  (:Pressed
    (bind _location (Timeline|MoveShelf PlayFromStart)
      (:Update
        (Transformation|SetWorldLocation (Variables|Default|GetShelf) (Math|Vector|Lerp(Vector) (Variables|Default|GetStartPos) (Variables|Default|GetEndPos) _location) false false)))))

(fn ConstructionScript)