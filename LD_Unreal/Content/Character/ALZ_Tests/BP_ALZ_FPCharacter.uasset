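; First-person player character with axis-driven look and movement, sprint, crouch, and world keypad clicks through WidgetInteraction.
; Sprint and crouch timelines interpolate walk speed; crouch also resizes the capsule and lowers the camera, replacing built-in Crouch.
; Releasing crouch, or pressing it while sprinting, sets a Standup flag.
; While flagged, Tick sphere-traces overhead and reverses the crouch timeline when clear, clearing the flag on timeline finish.
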(event Custom|Standup
  (bind _capsulecomponent (Variables|Collision|GetCapsuleComponent))
  (bind _returnvalue (Transformation|GetWorldLocation _capsulecomponent))
  ;[0.3872 0.4056 1] Check space above the character to standup
  (bind _returnvalue_2 (Collision|SphereTraceByChannel (+ _returnvalue "0.000000,0.000000,30.000000") (+ _returnvalue "0.000000,0.000000,90.000000") 65.0 "TraceTypeQuery1" false 0 "ForDuration"))
  (if (not _returnvalue_2)
    ;[0.3872 0.4056 1] Crouch
    (bind _crouch (Timeline|Timeline_Crouch Reverse)
      (:Update
        (Components|Capsule|SetCapsuleHalfHeight (Variables|Collision|GetCapsuleComponent) (Math|Float|Lerp 96.0 48.0 _crouch) true)
        (Transformation|SetRelativeLocation (Variables|Default|GetFirstPersonCamera) (Math|Vector|MakeVector 0.0 0.0 (* (Math|Float|Lerp 96.0 48.0 _crouch) 0.67)) false false)
        (Variables|/Script/Engine.CharacterMovementComponent|SetMaxWalkSpeed (Variables|Character|GetCharacterMovement) (Math|Float|Lerp 3.5e+02 1.5e+02 _crouch)))
      (:Finished
        (Variables|Default|SetStandup? false)))))

(event EventTick
  (params (DeltaSeconds :type Float%20%28single-precision%29))
  ;[0.3872 0.4056 1] Check crouch input
  (Utilities|FlowControl|Sequence
    (:then_0
      (if (Variables|Default|GetStandup?)
        (CallFunction|Standup)))))

(event Input|ActionEvents|InputActionCrouch
  (params (Key :type Key%20Structure :default "None"))
  ;[0.3872 0.4056 1] Crouch
  (:Pressed
    (if (Variables|Default|GetSprinting?)
      (Variables|Default|SetStandup? true :!label _label)
      (else
        (Variables|Default|SetStandup? false)
        (bind _crouch (Timeline|Timeline_Crouch Play)
          (:Update
            (Components|Capsule|SetCapsuleHalfHeight (Variables|Collision|GetCapsuleComponent) (Math|Float|Lerp 96.0 48.0 _crouch) true)
            (Transformation|SetRelativeLocation (Variables|Default|GetFirstPersonCamera) (Math|Vector|MakeVector 0.0 0.0 (* (Math|Float|Lerp 96.0 48.0 _crouch) 0.67)) false false)
            (Variables|/Script/Engine.CharacterMovementComponent|SetMaxWalkSpeed (Variables|Character|GetCharacterMovement) (Math|Float|Lerp 3.5e+02 1.5e+02 _crouch)))
          (:Finished
            (Variables|Default|SetStandup? false))))))
  (:Released
    (goto _label)))

(event Input|ActionEvents|InputActionCrouch
  (params (Key :type Key%20Structure :default "None"))
  ;[1 1 1] Crouch
)

(event Input|ActionEvents|InputActionSprint
  (params (Key :type Key%20Structure :default "None"))
  ;[1 0.3419 0.3515] Sprint
  (:Pressed
    (Variables|Default|SetSprinting? true)
    (bind _sprint (Timeline|Timeline_Sprint Play)
      (:Update
        (Variables|/Script/Engine.CharacterMovementComponent|SetMaxWalkSpeed (Variables|Character|GetCharacterMovement) (Math|Float|Lerp 3.5e+02 6e+02 _sprint)))))
  (:Released
    (Variables|Default|SetSprinting? false)
    (Timeline|Timeline_Sprint Reverse)))

(event Input|ActionEvents|InputActionDigitInteraction
  (params (Key :type Key%20Structure :default "None"))
  (bind _widgetinteraction (Variables|Default|GetWidgetInteraction))
  ;[0.902 0.7765 0.8039] Permet de cliquer sur le Keypad dans l'environnement
  (:Pressed
    (Class|WidgetInteractionComponent|PressPointerKey _widgetinteraction "LeftMouseButton"))
  (:Released
    (Class|WidgetInteractionComponent|ReleasePointerKey _widgetinteraction "LeftMouseButton")))

(event Input|AxisEvents|InputAxisLookUpDown
  (params (AxisValue :type Float%20%28single-precision%29))
  ;[1 0.9019 0.4385] CameraControl
  (Pawn|Input|AddControllerPitchInput (* AxisValue (Utilities|Time|GetWorldDeltaSeconds) (Variables|Default|GetTurnRatePitch))))

(event Input|AxisEvents|InputAxisLookLeftRight
  (params (AxisValue :type Float%20%28single-precision%29))
  ;[1 0.9019 0.4385] CameraControl
  (Pawn|Input|AddControllerYawInput (* (Utilities|Time|GetWorldDeltaSeconds) AxisValue (Variables|Default|GetTurnRateYaw))))

(event Input|AxisEvents|InputAxisMoveRightLeft
  (params (AxisValue :type Float%20%28single-precision%29))
  ;[1 0.3419 0.3515] PlayerMovement
  (Pawn|Input|AddMovementInput (Transformation|GetActorRightVector) AxisValue false))

(event Input|AxisEvents|InputAxisMoveForwardBackward
  (params (AxisValue :type Float%20%28single-precision%29))
  ;[1 0.3419 0.3515] PlayerMovement
  (Pawn|Input|AddMovementInput (Transformation|GetActorForwardVector) AxisValue false))

(fn ConstructionScript)