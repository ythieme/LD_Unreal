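; Ceiling light actor that flickers its rect light at random intervals, with sound.
; BeginPlay spawns a static electricity sound at the mesh location.
; Tick drives a latent Delay chain that waits random whole seconds below MaxTimeBetweenFlick, briefly hides the light, then restores it and plays a flicker cue at the mesh.
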(event EventBeginPlay
  (Audio|SpawnSoundatLocation "/Game/Draft/Sound/StaticElectricity_Cue.StaticElectricity_Cue" (Transformation|GetWorldLocation (Variables|Debug|GetStaticMeshComponent)) "0, 0, 0" 1.0 1.0 0.0 0 0))

(event EventTick
  (params (DeltaSeconds :type Float%20%28single-precision%29))
  (bind _rectlight (Variables|Default|GetRectLight))
  ;[1 1 1] Fait clignoter la lumière en suivant une intervalle aléatoire
  (Utilities|FlowControl|Delay (Math|Conversions|ToFloat(Integer) (Math|Random|RandomInteger (Variables|Default|GetMaxTimeBetweenFlick))))
  (Rendering|SetVisibility _rectlight false false)
  (Utilities|FlowControl|Delay 0.2)
  (Rendering|SetVisibility _rectlight true false)
  (Audio|PlaySoundatLocation "/Game/Draft/Sound/Light_Flicker_Cue.Light_Flicker_Cue" (Transformation|GetWorldLocation (Variables|Debug|GetStaticMeshComponent)) "0, 0, 0" 1.0 1.0 0.0 0 0 0 0))

(fn ConstructionScript)